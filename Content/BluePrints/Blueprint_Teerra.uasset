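; Blueprint_Teerra is an orbiting body, apparently Earth by its name, that circles the location of a ActorCentro actor.
; Each tick it rotates its offset from the previous centre around Axis at Velocidade degrees per second, then re-adds the current centre to follow moving targets.
; Before each step, OrthoganalizeAxis uses a double cross product to keep Axis normalized and perpendicular to that offset.
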(event `OrthoganalizeAxis`
  (bind _returnvalue (- (`self.K2_GetActorLocation`) (`self.Antigo Centro`)))
  (set `self.Axis` (`KismetMathLibrary.Normal` (`KismetMathLibrary.Cross_VectorVector` _returnvalue (`KismetMathLibrary.Cross_VectorVector` (`self.Axis`) _returnvalue)))))

(event `self.ReceiveBeginPlay`
  (`|ExecutionSequence`
    (:`then_0`
      (bind _actor_centro (`self.Actor Centro`)
        (:`then`
          (set `self.Localização do centro` (`self.K2_GetActorLocation` _actor_centro)))
        (:`else`)))
    (:`then_1`
      (set `self.Antigo Centro` (`self.Localização do centro`)))))

(event `self.ReceiveTick`
  (params (DeltaSeconds :type "Float (single-precision)"))
  (`|ExecutionSequence`
    (:`then_0`
      (bind _actor_centro (`self.Actor Centro`)
        (:`then`
          (set `self.Localização do centro` (`self.K2_GetActorLocation` _actor_centro)))
        (:`else`)))
    (:`then_1`
      (`self.OrthoganalizeAxis`)
      (`self.K2_SetActorLocation` (+ (`KismetMathLibrary.RotateAngleAxis` (- (`self.K2_GetActorLocation`) (`self.Antigo Centro`)) (* DeltaSeconds (`self.Velocidade`)) (`self.Axis`)) (`self.Localização do centro`)))
      (set `self.Antigo Centro` (`self.Localização do centro`)))))

(fn `UserConstructionScript`)